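; Traffic car Blueprint, apparently for looping vehicles, with much of its driving logic left empty or disconnected.
; Tick calls auto-steering, but the steering, drive and recolor events are empty, and the look-at steering math is unused.
; Tag-checked overlaps teleport the car to a fixed point at "ElDestructor2" and call drive when "Vehiculo2" leaves.
; Hitting "barreras" calls a print-only brake, then a reverse event that sets throttle.
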(event `C_Velocity`
  ;[1 1 1] Clampear Velocity
)

(event `self.ReceiveTick`
  (params (DeltaSeconds :type "Float (single-precision)"))
  ;[1 1 1] LA MAGIA
  (`self.Auto_Doblar`)
  (if (== 0.0 1.0)
    (`self.Andar`)))

(event `self.Box.OnComponentBeginOverlap`
  (params (OverlappedComponent :type "PrimitiveComponent Object Reference") (OtherActor :type "Actor Object Reference") (OtherComp :type "PrimitiveComponent Object Reference") (OtherBodyIndex :type Integer) (bFromSweep :type Boolean) (SweepResult :type "HitResult Structure (by ref)"))
  ;[1 1 1] Frenar por colision con otros Vehiculos
  (if (`self.ActorHasTag` OtherActor "Vehiculo2")
    (`KismetSystemLibrary.PrintString` "")
    (else
      (`KismetSystemLibrary.PrintString` "")))
  (if (`self.ActorHasTag` OtherActor "ElDestructor2")
    (`self.K2_TeleportTo` (1294.0 26581.0 21.0) (struct :`Yaw` -80.0))
    (`self.ChanheColor`)
    (else
      (`KismetSystemLibrary.PrintString` ""))))

(event `Auto_Doblar`
  ;[1 1 1] DOBLAR
)

(event `Frenar`
  ;[1 1 1] FRENAR
  (`KismetSystemLibrary.PrintString` ""))

(event `ChanheColor`
  ;[1 1 1] CAMBIO DE COLOR
)

(event `self.Box.OnComponentEndOverlap`
  (params (OverlappedComponent :type "PrimitiveComponent Object Reference") (OtherActor :type "Actor Object Reference") (OtherComp :type "PrimitiveComponent Object Reference") (OtherBodyIndex :type Integer))
  ;[1 1 1] Partir despues de una colision
  (if (`self.ActorHasTag` OtherActor "Vehiculo2")
    (`KismetSystemLibrary.PrintString` "")
    (`self.Andar`)
    (else
      (`KismetSystemLibrary.PrintString` ""))))

(event `self.Mesh.OnComponentBeginOverlap`
  (params (OverlappedComponent :type "PrimitiveComponent Object Reference") (OtherActor :type "Actor Object Reference") (OtherComp :type "PrimitiveComponent Object Reference") (OtherBodyIndex :type Integer) (bFromSweep :type Boolean) (SweepResult :type "HitResult Structure (by ref)"))
  ;[1 1 1] COLISION CON BARRERAS
  (if (`self.ActorHasTag` OtherActor "barreras")
    (`KismetSystemLibrary.PrintString` "")
    (`self.Frenar`)
    (`self.marchaAtras`)))

(event `Andar`
  ;[1 1 1] ANDAR
)

(event `marchaAtras`
  ;[1 1 1] MARCHA ATRAS
  (set `self.Throttle` 3.0))

(fn `UserConstructionScript`)